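; stateBP is an actor that displays a state mesh, labeled with the mesh's object name and colored by a numeric StateValue.
; The construction script assigns StateMesh and picks a blue, green, yellow or red material through descending value thresholds.
; It then snaps Bar to Loc's relative location, skipping material and move for negative values.
; The event graph has no active logic, only empty events and an unconnected delayed Bar move.
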(event EventBeginPlay)

(event Collision|EventActorBeginOverlap
  (params (OtherActor :type Actor%20Object%20Reference)))

(event EventTick
  (params (DeltaSeconds :type Float%20%28single-precision%29)))

(fn ConstructionScript
  (bind _statevalue (Variables|Default|GetstateValue))
  (Rendering|Components|TextRender|SetText (Variables|Default|GetTextRender2) (Utilities|Text|ToText(String) (Utilities|GetObjectName (Variables|Default|GetstateMesh))))
  (Components|StaticMesh|SetStaticMesh (Variables|Default|GetstateMap) (Variables|Default|GetstateMesh))
  (if (>= _statevalue 2.5e+03)
    (Variables|Default|Setcolor "/Game/assets/Material/Blue.Blue")
    (Rendering|Material|SetMaterial (Variables|Default|GetstateMap) 0 (Variables|Default|Getcolor) :!label _label)
    (Transformation|SetRelativeLocation (Variables|Default|Getbar) (Variables|/Script/Engine.SceneComponent|GetRelativeLocation (Variables|Default|Getloc)) false false)
    (elif (>= _statevalue 1.5e+03)
      (Variables|Default|Setcolor "/Game/assets/Material/Green.Green")
      (goto _label)
      (elif (>= _statevalue 1e+03)
        (Variables|Default|Setcolor "/Game/assets/Material/Yellow.Yellow")
        (goto _label)
        (elif (>= _statevalue 0.0)
          (Variables|Default|Setcolor "/Game/assets/Material/RedL.RedL")
          (goto _label))))))